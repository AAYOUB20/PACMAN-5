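; Pac-Man player pawn Blueprint that plays sound feedback when its Collider overlaps a ghost (PhantomPawn).
; IsSuperPowerEnabled selects the ghost-eaten sound or the death sound, both played as 2D audio, and Consumed is then set to true.
; The Consumed check has empty branches, and the graph contains no movement, scoring or death handling.
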(event OnComponentBeginOverlap(Collider)
  (params (OverlappedComponent :type Primitive%20Component%20Object%20Reference) (OtherActor :type Actor%20Object%20Reference) (OtherComp :type Primitive%20Component%20Object%20Reference) (OtherBodyIndex :type Integer) (bFromSweep :type Boolean) (SweepResult :type Hit%20Result%20Structure%20%28by%20ref%29))
  (Utilities|Casting|CastToPhantomPawn OtherActor)
  (if (not (Variables|Default|GetbConsumed))
    _
    (else
      _))
  (bind _returnvalue (Class|PacmanPawn|IsSuperPowerEnabled))
  (if _returnvalue
    (Audio|PlaySound2D "/Game/Pacman_Sounds/eat_ghost.eat_ghost" 1.0 1.0 0.0 0 self)
    (else
      (Audio|PlaySound2D "/Game/Pacman_Sounds/death.death" 1.0 1.0 0.0 0 self)))
  (Variables|Default|SetbConsumed true))

(event EventBeginPlay)

(event Collision|EventActorBeginOverlap
  (params (OtherActor :type Actor%20Object%20Reference)))

(event EventTick
  (params (DeltaSeconds :type Float%20%28single-precision%29)))

(fn ConstructionScript)